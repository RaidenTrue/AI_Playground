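; Behavior tree service that sets an IsStuck blackboard flag for the controlled AI pawn.
; On activation it stores the pawn's location in LastLocation.
; Each tick, only when the pawn's distance from the LastLoc value exceeds DistanceThreshold, it sets IsStuck by whether TimeNotMoved exceeds StuckTimeThreshold.
; It never updates TimeNotMoved or refreshes the stored location during ticks.
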(event `self.ReceiveActivationAI`
  (params (OwnerController :type "AIController Object Reference") (ControlledPawn :type "Pawn Object Reference"))
  (`BTFunctionLibrary.SetBlackboardValueAsVector` (`self.LastLocation`) (`Actor.K2_GetActorLocation` ControlledPawn)))

(event `self.ReceiveTickAI`
  (params (OwnerController :type "AIController Object Reference") (ControlledPawn :type "Pawn Object Reference") (DeltaSeconds :type "Float (single-precision)"))
  (bind _returnvalue (`AIBlueprintHelperLibrary.GetBlackboard` ControlledPawn))
  (if (> (`KismetMathLibrary.Vector_Distance` (`Actor.K2_GetActorLocation` ControlledPawn) (`BlackboardComponent.GetValueAsVector` _returnvalue (`self.LastLoc`))) (`self.DistanceThreshold`))
    (if (> (`BlackboardComponent.GetValueAsFloat` _returnvalue (`self.TimeNotMoved`)) (`self.StuckTimeThreshold`))
      (`BlackboardComponent.SetValueAsBool` _returnvalue (`self.IsStuck`) true)
      (else
        (`BlackboardComponent.SetValueAsBool` _returnvalue (`self.IsStuck`) false)))))