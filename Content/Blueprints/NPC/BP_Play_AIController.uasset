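; BP_Play_AIController is an NPC AI controller that runs the BT_BasicAI behavior tree on possession.
; Its AI Perception updates feed the TargetActor blackboard key, storing each sensed actor and clearing the ForgetTarget timer by name.
; A failed sense starts that timer with the LoseInterest delay only if the actor differs from the stored target.
; When the timer fires, ForgetTarget clears the key.
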(event `self.ReceiveBeginPlay`)

(event `self.ReceivePossess`
  (params (PossessedPawn :type "Pawn Object Reference"))
  (`self.RunBehaviorTree` "/Game/Blueprints/AIBehavior/BT_BasicAI.BT_BasicAI"))

(event `self.AIPerception.OnTargetPerceptionUpdated`
  (params (Actor :type "Actor Object Reference") (Stimulus :type "AIStimulus Structure"))
  (bind _returnvalue (`AIBlueprintHelperLibrary.GetBlackboard` null))
  (if (`.bSuccessfullySensed` (break `AIStimulus` Stimulus))
    (`KismetSystemLibrary.K2_ClearTimer` null "ForgetTarget")
    (`BlackboardComponent.SetValueAsObject` _returnvalue (`self.TargetActor`) Actor)
    (elif (!= Actor (`BlackboardComponent.GetValueAsObject` _returnvalue (`self.TargetActor`)))
      (bind _returnvalue_2 (`KismetSystemLibrary.K2_SetTimerDelegate` (delegate `ForgetTarget`) (`self.LoseInterest`)))
      (set `self.LoseInterestHandle` _returnvalue_2))))

(event `ForgetTarget`
  (`BlackboardComponent.ClearValue` (`AIBlueprintHelperLibrary.GetBlackboard` null) (`self.TargetActor`)))

(fn `UserConstructionScript`)